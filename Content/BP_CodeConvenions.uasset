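; BP_CodeConvenions is a reference Blueprint that demonstrates the team's coding and commenting conventions rather than gameplay.
; Its EventGraph holds unconnected Print String and Delay chains, each labeled with a team member's name, with sample comments on the first.
; Placeholder impure and pure functions that return false, plus an empty example macro, serve as examples of each graph type.
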(fn ConstructionScript)

(fn ExampleFunction
  (params (exampleInput :type Boolean))
  (return false))

(fn ExampleFunction(Pure)
  (params (exampleInput :type Boolean))
  (return false))