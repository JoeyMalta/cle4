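; Player controller Blueprint that toggles the pause menu from the IA_PauseGame Enhanced Input action.
; A FlipFlop alternates between creating a fresh WBP_PauseMenu with the cursor shown in Game and UI input mode, and removing it to restore hidden-cursor, game-only input with viewport focus.
; The toggle handles only menu, cursor and input mode, with no call here to pause the game itself.
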(event Input|EnhancedActionEvents|EnhancedInputActionIA_PauseGame
  (params (ActionValue :type Boolean) (ElapsedSeconds :type Float%20%28double-precision%29) (TriggeredSeconds :type Float%20%28double-precision%29) (InputAction :type Input%20Action%20Object%20Reference :default "/Game/Game/UI/Jani/Inputs/IA_PauseGame.IA_PauseGame"))
  (bind _returnvalue (Game|GetPlayerController 0))
  (bind _returnvalue_2 (Game|GetPlayerController 0))
  ;[0.15 0.15 0.15 0.5] Press Pause Button
  (:Started
    (Utilities|FlowControl|FlipFlop
      (:A
        ;[0.15 0.15 0.15 0.5] Create Pause Widget
        (bind _returnvalue_3 (UserInterface|CreateWidget "/Game/Game/UI/Jani/UI/Widgets/WBP_PauseMenu.WBP_PauseMenu_C"))
        (UserInterface|Viewport|AddtoViewport _returnvalue_3 0)
        ;[0.15 0.15 0.15 0.5] Show the Mouse On Pause Menu
        (Variables|/Script/Engine.PlayerController|SetbShowMouseCursor _returnvalue_2 true)
        ;[0.15 0.15 0.15 0.5] unlock the mouse from player
        (Input|SetInputModeGameandUI _returnvalue_2 0 "DoNotLock" true false))
      (:B
        ;[0.15 0.15 0.15 0.5] Remove Pause Widget
        (Widget|RemovefromParent _returnvalue_3)
        ;[0.15 0.15 0.15 0.5] hide Mouse From Screen
        (Variables|/Script/Engine.PlayerController|SetbShowMouseCursor _returnvalue false)
        ;[0.15 0.15 0.15 0.5] Focus mouse in game again so player can look around
        (Input|SetInputModeGameOnly _returnvalue false)
        (Class|WidgetBlueprintLibrary|SetFocustoGameViewport)))))

(fn ConstructionScript)