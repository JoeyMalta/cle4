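; First-person player character handling Enhanced Input movement, look, jump and sprint, plus interaction with world actors.
; A camera line trace feeds interface messages: observe on Tick, interact on pick-up and open on interact.
; Pick-up, interact and drop inputs route to the held actor when one exists.
; Timelines bob the held-object socket while walking, gated by paired DoOnce nodes, and bounce a child actor whose visibility NumPad 5 toggles.
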(event Input|EnhancedActionEvents|EnhancedInputActionIA_Look
  (params (ActionValue :type Vector%202D%20Structure) (ElapsedSeconds :type Float%20%28double-precision%29) (TriggeredSeconds :type Float%20%28double-precision%29) (InputAction :type Input%20Action%20Object%20Reference :default "/Game/Game/Player/Input/InputAction/IA_Look.IA_Look"))
  ;[0.2346 0.5457 0.6584 0.502] Player Mouse Movement
  (Pawn|Input|AddControllerYawInput (.x ActionValue))
  (Pawn|Input|AddControllerPitchInput (.y ActionValue)))

(event Input|EnhancedActionEvents|EnhancedInputActionIA_Move
  (params (ActionValue :type Vector%202D%20Structure) (ElapsedSeconds :type Float%20%28double-precision%29) (TriggeredSeconds :type Float%20%28double-precision%29) (InputAction :type Input%20Action%20Object%20Reference :default "/Game/Game/Player/Input/InputAction/IA_Move.IA_Move"))
  (bind _returnvalue (Pawn|GetControlRotation :!class /Script/Engine.Pawn))
  ;[0.2346 0.5457 0.6584 0.502] Player Movement
  (:Triggered
    (CallFunction|PlayWalkingAnimation)
    (Pawn|Input|AddMovementInput (Math|Vector|GetRightVector (Math|Rotator|MakeRotator (.roll _returnvalue) 0.0 (.yaw _returnvalue))) (.x ActionValue) false)
    (Pawn|Input|AddMovementInput (Math|Vector|GetForwardVector (Math|Rotator|MakeRotator 0.0 0.0 (.yaw (Pawn|GetControlRotation :!class /Script/Engine.Pawn)))) (.y ActionValue) false))
  (:Completed
    (CallFunction|StopWalkingAnimation)))

(event Input|EnhancedActionEvents|EnhancedInputActionIA_Jump
  (params (ActionValue :type Boolean) (ElapsedSeconds :type Float%20%28double-precision%29) (TriggeredSeconds :type Float%20%28double-precision%29) (InputAction :type Input%20Action%20Object%20Reference :default "/Game/Game/Player/Input/InputAction/IA_Jump.IA_Jump"))
  ;[0.2346 0.5457 0.6584 0.502] Jumping
  (:Triggered
    (Character|Jump))
  (:Completed
    (Character|StopJumping)))

(event Input|EnhancedActionEvents|EnhancedInputActionIA_Sprint
  (params (ActionValue :type Boolean) (ElapsedSeconds :type Float%20%28double-precision%29) (TriggeredSeconds :type Float%20%28double-precision%29) (InputAction :type Input%20Action%20Object%20Reference :default "/Game/Game/Player/Input/InputAction/IA_Sprint.IA_Sprint"))
  (bind _charactermovement (Variables|Character|GetCharacterMovement))
  ;[0.2346 0.5457 0.6584 0.502] Sprinting
  (:Triggered
    (Variables|/Script/Engine.CharacterMovementComponent|SetMaxWalkSpeed _charactermovement 9e+02))
  (:Completed
    (Variables|/Script/Engine.CharacterMovementComponent|SetMaxWalkSpeed _charactermovement 6e+02)))

(event EventBeginPlay
  ;[0.2346 0.5457 0.6584 0.502] Add IMC
  (bind _asplayer_controller (Utilities|Casting|CastToPlayerController (Pawn|GetController)))
  (Utilities|IsValid _asplayer_controller
    (:Is%20Valid
      (Input|AddMappingContext (PlayerController|LocalPlayerSubsystems|GetEnhancedInputLocalPlayerSubsystem _asplayer_controller) "/Game/Game/Player/Input/InputActionMapping/IMC_Player.IMC_Player" 0 "(bIgnoreAllPressedKeysUntilRelease=True,bForceImmediately=False,bNotifyUserSettings=False)")
      ;[0.4621 1 0.4125] Add Walk Anim
      (Components|Timeline|SetPlayRate (Variables|Default|GetWalkAnimation) (/ 1.0 0.6)))))

(event Custom|playWalkingAnimation
  ;[0.4604 1 0.414] The actual animation of the object that is picked up.
  (Utilities|FlowControl|Sequence
    (:then_0
      (Utilities|FlowControl|DoOnce false
        (:Completed
          (bind (_direction _vector) (Timeline|WalkAnimation Play)
            (:Update
              (Transformation|SetRelativeLocation (Variables|Default|Getattach_socket) _vector false false))
            (:Finished
              (switch Utilities|FlowControl|Switch|SwitchonETimelineDirection _direction
                (:Forward
                  (Timeline|WalkAnimation ReverseFromEnd))
                (:Backward
                  (Timeline|WalkAnimation PlayFromStart))))))))
    (:then_1
      (Utilities|FlowControl|DoOnce false) ; enters at Reset
    )))

(event Custom|stopWalkingAnimation
  ;[0.4604 1 0.414] The actual animation of the object that is picked up.
  (Utilities|FlowControl|Sequence
    (:then_0
      (Utilities|FlowControl|DoOnce false
        (:Completed
          (bind (_direction _vector) (Timeline|WalkAnimation Stop)
            (:Update
              (Transformation|SetRelativeLocation (Variables|Default|Getattach_socket) _vector false false))
            (:Finished
              (switch Utilities|FlowControl|Switch|SwitchonETimelineDirection _direction
                (:Forward
                  (Timeline|WalkAnimation ReverseFromEnd))
                (:Backward
                  (Timeline|WalkAnimation PlayFromStart))))))))
    (:then_1
      (Utilities|FlowControl|DoOnce false) ; enters at Reset
    )))

(event Input|EnhancedActionEvents|EnhancedInputActionIA_PickUp
  (params (ActionValue :type Boolean) (ElapsedSeconds :type Float%20%28double-precision%29) (TriggeredSeconds :type Float%20%28double-precision%29) (InputAction :type Input%20Action%20Object%20Reference :default "/Game/Game/Player/Input/InputAction/IA_PickUp.IA_PickUp"))
  ;[0.4604 1 0.414] Interact with Actors in the world using Linetracing. Interface is responsable for handeling the requests
  (:Started
    (Variables|Default|GetBP_HeldActor
      (:then
        (bind _outhit (CallFunction|LinetracefromCamera))
        (Class|BIInteractInterface|InterfaceInteract(Message) (Variables|Default|GetBP_HeldActor) self true _outhit))
      (:else
        (bind (_returnvalue _outhit_2) (CallFunction|LinetracefromCamera))
        (if _returnvalue
          (Class|BIInteractInterface|InterfaceInteract(Message) (.HitActor (Collision|BreakHitResult _outhit_2)) self false _outhit_2))))))

(event Input|EnhancedActionEvents|EnhancedInputActionIA_Interact
  (params (ActionValue :type Boolean) (ElapsedSeconds :type Float%20%28double-precision%29) (TriggeredSeconds :type Float%20%28double-precision%29) (InputAction :type Input%20Action%20Object%20Reference :default "/Game/Game/Player/Input/InputAction/IA_Interact.IA_Interact"))
  ;[0.4508 0.9792 0.4054] [Joey] Controleert via een line trace welk object de speler aankijkt en activeert de interactie wanneer een geldig object wordt geraakt.
  (:Started
    (Variables|Default|GetBP_HeldActor
      (:then
        (bind _outhit (CallFunction|LinetracefromCamera))
        (Class|BIInteractInterface|InterfaceOpen(Message) (Variables|Default|GetBP_HeldActor) true _outhit))
      (:else
        (bind (_returnvalue _outhit_2) (CallFunction|LinetracefromCamera))
        (if _returnvalue
          (Class|BIInteractInterface|InterfaceOpen(Message) (.HitActor (Collision|BreakHitResult _outhit_2)) false _outhit_2))))))

(event Input|EnhancedActionEvents|EnhancedInputActionIA_Drop
  (params (ActionValue :type Boolean) (ElapsedSeconds :type Float%20%28double-precision%29) (TriggeredSeconds :type Float%20%28double-precision%29) (InputAction :type Input%20Action%20Object%20Reference :default "/Game/Game/Player/Input/InputAction/IA_Drop.IA_Drop"))
  ;[0.4621 1 0.4125] Drop the held actor
  (:Started
    (bind _bp_heldactor (Variables|Default|GetBP_HeldActor)
      (:then
        (Class|BIInteractInterface|InterfaceDrop(Message) _bp_heldactor false))
      (:else))))

(event EventTick
  (params (DeltaSeconds :type Float%20%28single-precision%29))
  ;[0.4508 0.9792 0.4054] [Joey] Detecteert continu interactable objecten waar de speler naar kijkt en werkt de interactie-UI hierop bij.
  (Variables|Default|GetBP_HeldActor
    (:then
      (bind (_returnvalue _outhit) (CallFunction|LinetracefromCamera))
      (if _returnvalue
        (Class|BIInteractInterface|InterfaceObserve(Message) (.HitActor (Collision|BreakHitResult _outhit)) self true _outhit)))
    (:else
      (bind (_returnvalue_2 _outhit_2) (CallFunction|LinetracefromCamera))
      (if _returnvalue_2
        (Class|BIInteractInterface|InterfaceObserve(Message) (.HitActor (Collision|BreakHitResult _outhit_2)) self false _outhit_2)))))

(event Input|KeyboardEvents|NumPadFive
  (params (Key :type Key%20Structure))
  ;[0.6201 0.42 1] [shayenne]
  (:Pressed
    (Utilities|FlowControl|FlipFlop
      (:A
        (Development|SetHiddeninGame (Variables|Default|GetChildActor) true false)
        (Components|Timeline|SetPlayRate (Variables|Default|GetBounceAnim) (/ 1.0 0.1))
        (bind _newtrack_1 (Timeline|BounceAnim PlayFromStart)
          (:Update
            (Transformation|SetRelativeLocation (Variables|Default|GetChildActor) _newtrack_1 false false))))
      (:B
        (Development|SetHiddeninGame (Variables|Default|GetChildActor) false false)
        (Components|Timeline|SetPlayRate (Variables|Default|GetBounceAnim) (/ 1.0 0.1))
        (Timeline|BounceAnim ReverseFromEnd)))))

(fn ConstructionScript)

(fn LinetracefromCamera
  (bind _camera (Variables|Default|GetCamera))
  (bind _returnvalue (Transformation|GetWorldLocation _camera))
  (bind (_outhit _returnvalue_2) (Collision|LineTraceByChannel _returnvalue (+ _returnvalue (* (Math|Vector|GetForwardVector _camera) (Variables|Default|GetTraceLength))) "TraceTypeQuery1" false 0 "None"))
  (return _returnvalue_2 _outhit))