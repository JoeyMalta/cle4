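; BP_CardboardBox is a cardboard box that the player can pick up, drop, open and close.
; On BeginPlay it shows one of three random Dutch content labels on its text render.
; Interact attaches the mesh to the player's socket without physics or collision and registers it as HeldActor; drop detaches and restores both.
; Open uses a FlipFlop to swap between open and closed meshes.
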(event EventInterfaceOpen
  (bind _sm_cardboardbox (Variables|Default|GetSM_Cardboardbox))
  (Utilities|FlowControl|FlipFlop
    (:A
      (Components|StaticMesh|SetStaticMesh _sm_cardboardbox "/Game/Mega_Survival_Tools/Models/SM_Cardboard_Box_01_Open.SM_Cardboard_Box_01_Open"))
    (:B
      (Components|StaticMesh|SetStaticMesh _sm_cardboardbox "/Game/Mega_Survival_Tools/Models/SM_Cardboard_Box_01_Closed.SM_Cardboard_Box_01_Closed"))))

(event EventBeginPlay
  (Rendering|Components|TextRender|SetText (Variables|Default|GetTextRender) (Utilities|Select :Index (Math|Random|RandomIntegerinRange 0 2) :Option%200 (Utilities|Text|FormatText "Medicijnen") :Option%201 (Utilities|Text|FormatText "Kauwgom") :Option%202 (Utilities|Text|FormatText "Banaan"))))

(event EventInterfaceInteract
  (params (actor :type Actor%20Object%20Reference))
  ;[0.4604 1 0.414] Comment
  (bind _asbp_player (Utilities|Casting|CastToBP_Player actor))
  (Variables|Default|SetAs%20BP%20Player _asbp_player)
  (Physics|SetSimulatePhysics (Variables|Default|GetSM_Cardboardbox) false)
  (Transformation|AttachComponentToComponent (Variables|Default|GetSM_Cardboardbox) (Variables|/Game/Game/Player/BP_Player.BP_Player_C|Getattach_socket _asbp_player) "None" "SnapToTarget" "SnapToTarget" "KeepRelative" true)
  (Collision|SetCollisionEnabled (Variables|Default|GetSM_Cardboardbox) "NoCollision")
  (Variables|/Game/Game/Player/BP_Player.BP_Player_C|SetheldActor _asbp_player self))

(event EventInterfaceDrop
  (Collision|SetCollisionEnabled (Variables|Default|GetSM_Cardboardbox) "QueryAndPhysics")
  (Transformation|DetachFromActor self "KeepWorld" "KeepWorld" "KeepWorld")
  (Physics|SetSimulatePhysics (Variables|Default|GetSM_Cardboardbox) true))

(fn ConstructionScript
  (|CallParentFunction))