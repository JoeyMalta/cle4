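; Intro booklet actor that the player pages through once the HUD intro sequence finishes.
; Shoulder buttons or E/Q drive a FlipPage timeline that rotates the current page with a turn sound, using DoOnce gates to serialize flips.
; Advancing past the last page rapidly flips back via a delayed-loop macro, disables input and launches the pieces with physics.
; It then spawns and drops BP_BookletTutorial, starts BP_DistributionManager's distribution and destroys itself.
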(event OnComponentHit(BackCover)
  (params (HitComponent :type Primitive%20Component%20Object%20Reference) (OtherActor :type Actor%20Object%20Reference) (OtherComp :type Primitive%20Component%20Object%20Reference) (NormalImpulse :type Vector :default "0, 0, 0") (Hit :type Hit%20Result%20Structure%20%28by%20ref%29))
  ;[0.6201 0.42 1] [Shayenne]
  (Utilities|FlowControl|DoOnce false
    (:Completed
      (Utilities|FlowControl|Delay 0.5)
      (Audio|PlaySoundatLocation "/Game/Game/Actors/IntroBooklet/SFX/SFX_IntroBooketDrop.SFX_IntroBooketDrop" (Transformation|GetWorldLocation (Variables|Default|GetBackCover)) "0, 0, 0" 1.0 1.0 0.0 0 0 0 0))))

(event Custom|event_FlipBack
  (bind _frontcover (Variables|Default|GetFrontCover))
  (bind _frontcover_2 (Variables|Default|GetFrontCover))
  ;[0.6201 0.42 1] [Shayenne]
  (Utilities|ForLoopDelay 0 (Variables|Default|GetMaxPages) 0.05
    (:LoopBody
      (Components|Timeline|SetPlayRate (Variables|Default|GetFlipPage) (/ 1.0 0.05))
      (if (not (== (Variables|Default|GetpageCount) 0))
        (CallFunction|PlayAudio)
        (bind (_direction _alpha) (Timeline|FlipPage ReverseFromEnd)
          (:Update
            (Transformation|SetRelativeRotation (Utilities|Select :Index (Variables|Default|GetpageCount) :Option%200 0 :Option%201 _frontcover :Option%202 (Variables|Default|GetPage_Intro) :Option%203 (Variables|Default|GetPage_One) :Option%204 (Variables|Default|GetPage_Two)) (Math|Rotator|Lerp(Rotator) "90.000000,0.000000,0.000000" "90.000000,180.000000,0.000000" _alpha) false false)
            (if (== (Utilities|Select :Index (Variables|Default|GetpageCount) :Option%200 0 :Option%201 _frontcover :Option%202 (Variables|Default|GetPage_Intro) :Option%203 (Variables|Default|GetPage_One) :Option%204 (Variables|Default|GetPage_Two)) _frontcover)
              (switch Utilities|FlowControl|Switch|SwitchonETimelineDirection _direction
                (:Forward
                  (Transformation|SetRelativeLocation _frontcover_2 "-0.100000,0.000000,0.000000" false false))
                (:Backward
                  (Transformation|SetRelativeLocation _frontcover_2 "0.200000,0.000000,0.000000" false false)))))
          (:Finished
            (switch Utilities|FlowControl|Switch|SwitchonETimelineDirection _direction
              (:Forward
                (CallFunction|EventReset))
              (:Backward
                (bind _result (Math|Integer|DecrementInt (Variables|Default|GetpageCount))
                  (:%20%20
                    (Variables|Default|SetpageCount (Math|Integer|Clamp(Integer) _result 0 (Variables|Default|GetMaxPages)))
                    (CallFunction|EventReset)))))))))
    (:Completed
      (Input|DisableInput (Game|GetPlayerController 0))
      (Physics|SetSimulatePhysics (Variables|Default|GetBackCover) true)
      (Physics|AddImpulse (Variables|Default|GetBackCover) (* (Transformation|GetActorForwardVector (Game|GetPlayerCharacter 0)) 5e+02) "None" true)
      (Utilities|FlowControl|Delay 2.0)
      (bind _returnvalue (Game|SpawnActorfromClass "/Game/Game/Actors/Items/BP_BookletTutorial.BP_BookletTutorial_C" (Math|Transform|MakeTransform (Transformation|GetWorldLocation (Variables|Default|GetBackCover)) "0, 0, 0" "1.000000,1.000000,1.000000") "AlwaysSpawn" "MultiplyWithRoot" 0 0 0))
      (Default|InterfaceDrop _returnvalue false)
      (bind _returnvalue_2 (Actor|GetActorOfClass "/Game/Game/Actors/ConveyorBelt/BP_DistributionManager.BP_DistributionManager_C"))
      (Default|StartDistribution _returnvalue_2)
      (Actor|DestroyActor))))

(event Custom|event_Reset
  (bind _frontcover (Variables|Default|GetFrontCover))
  (bind _frontcover_2 (Variables|Default|GetFrontCover))
  ;[0.6201 0.42 1] [Shayenne]
  (Utilities|FlowControl|Sequence
    (:then_0
      (Utilities|FlowControl|DoOnce false) ; enters at Reset
    )
    (:then_1
      (Utilities|FlowControl|DoOnce false) ; enters at Reset
    )))

(event Custom|playAudio
  ;[0.6201 0.42 1] [Shayenne]
  (Audio|PlaySound2D (Utilities|Select :Index (Variables|Default|GetpageCount) :Option%200 0 :Option%201 "/Game/Game/Actors/IntroBooklet/SFX/SFX_PageTurn_01.SFX_PageTurn_01" :Option%202 "/Game/Game/Actors/IntroBooklet/SFX/SFX_PageTurn_02.SFX_PageTurn_02" :Option%203 "/Game/Game/Actors/IntroBooklet/SFX/SFX_PageTurn_03.SFX_PageTurn_03") 1.0 1.5 0.0 0 0))

(event Custom|event_IntroSequenceFinished_Event
  ;[0.6201 0.42 1] [Shayenne]
  (Input|EnableInput (Game|GetPlayerController 0)))

(event Custom|initBooklet
  ;[0.6201 0.42 1] [Shayenne]
  (Input|EnableInput (Game|GetPlayerController 0)))

(event Input|EnhancedActionEvents|EnhancedInputActionIA_Interact
  (params (ActionValue :type Boolean) (ElapsedSeconds :type Float%20%28double-precision%29) (TriggeredSeconds :type Float%20%28double-precision%29) (InputAction :type Input%20Action%20Object%20Reference :default "/Game/Game/Player/Input/InputAction/IA_Interact.IA_Interact"))
  ;[0.6201 0.42 1] [Shayenne]
)

(event EventBeginPlay
  ;[0.6201 0.42 1] [Shayenne]
  (bind _ashud_player_interface (Utilities|Casting|CastToHUD_PlayerInterface (HUD|GetHUD (Game|GetPlayerController 0))))
  (EventDispatchers|AssignEventIntroSequenceFinished _ashud_player_interface (delegate Custom|event_IntroSequenceFinished_Event))
  (Components|Timeline|SetPlayRate (Variables|Default|GetFlipPage) (/ 1.0 0.25)))

(event Input|KeyboardEvents|E
  (params (Key :type Key%20Structure))
  (bind _frontcover (Variables|Default|GetFrontCover))
  (bind _frontcover_2 (Variables|Default|GetFrontCover))
  ;[0.6201 0.42 1] [Shayenne]
  (:Pressed
    (Utilities|FlowControl|DoOnce false
      (:Completed
        (Development|PrintString "NEXT PAGE")
        (if (== (Variables|Default|GetpageCount) (- (Variables|Default|GetMaxPages) 1))
          (CallFunction|EventFlipBack)
          (else
            (bind _result (Math|Integer|IncrementInt (Variables|Default|GetpageCount))
              (:%20%20
                (Variables|Default|SetpageCount (Math|Integer|Clamp(Integer) _result 0 (Variables|Default|GetMaxPages)))
                (CallFunction|PlayAudio)
                (bind (_direction _alpha) (Timeline|FlipPage PlayFromStart)
                  (:Update
                    (Transformation|SetRelativeRotation (Utilities|Select :Index (Variables|Default|GetpageCount) :Option%200 0 :Option%201 _frontcover :Option%202 (Variables|Default|GetPage_Intro) :Option%203 (Variables|Default|GetPage_One) :Option%204 (Variables|Default|GetPage_Two)) (Math|Rotator|Lerp(Rotator) "90.000000,0.000000,0.000000" "90.000000,180.000000,0.000000" _alpha) false false)
                    (if (== (Utilities|Select :Index (Variables|Default|GetpageCount) :Option%200 0 :Option%201 _frontcover :Option%202 (Variables|Default|GetPage_Intro) :Option%203 (Variables|Default|GetPage_One) :Option%204 (Variables|Default|GetPage_Two)) _frontcover)
                      (switch Utilities|FlowControl|Switch|SwitchonETimelineDirection _direction
                        (:Forward
                          (Transformation|SetRelativeLocation _frontcover_2 "-0.100000,0.000000,0.000000" false false))
                        (:Backward
                          (Transformation|SetRelativeLocation _frontcover_2 "0.200000,0.000000,0.000000" false false)))))
                  (:Finished
                    (switch Utilities|FlowControl|Switch|SwitchonETimelineDirection _direction
                      (:Forward
                        (CallFunction|EventReset))
                      (:Backward
                        (bind _result_2 (Math|Integer|DecrementInt (Variables|Default|GetpageCount))
                          (:%20%20
                            (Variables|Default|SetpageCount (Math|Integer|Clamp(Integer) _result_2 0 (Variables|Default|GetMaxPages)))
                            (CallFunction|EventReset)))))))))))))))

(event Input|GamepadEvents|GamepadLeftShoulder
  (params (Key :type Key%20Structure))
  (bind _frontcover (Variables|Default|GetFrontCover))
  (bind _frontcover_2 (Variables|Default|GetFrontCover))
  ;[0.6201 0.42 1] [Shayenne]
  (:Pressed
    (Utilities|FlowControl|DoOnce false
      (:Completed
        (Development|PrintString "PREVIOUS PAGE")
        (if (not (== (Variables|Default|GetpageCount) 0))
          (CallFunction|PlayAudio)
          (bind (_direction _alpha) (Timeline|FlipPage ReverseFromEnd)
            (:Update
              (Transformation|SetRelativeRotation (Utilities|Select :Index (Variables|Default|GetpageCount) :Option%200 0 :Option%201 _frontcover :Option%202 (Variables|Default|GetPage_Intro) :Option%203 (Variables|Default|GetPage_One) :Option%204 (Variables|Default|GetPage_Two)) (Math|Rotator|Lerp(Rotator) "90.000000,0.000000,0.000000" "90.000000,180.000000,0.000000" _alpha) false false)
              (if (== (Utilities|Select :Index (Variables|Default|GetpageCount) :Option%200 0 :Option%201 _frontcover :Option%202 (Variables|Default|GetPage_Intro) :Option%203 (Variables|Default|GetPage_One) :Option%204 (Variables|Default|GetPage_Two)) _frontcover)
                (switch Utilities|FlowControl|Switch|SwitchonETimelineDirection _direction
                  (:Forward
                    (Transformation|SetRelativeLocation _frontcover_2 "-0.100000,0.000000,0.000000" false false))
                  (:Backward
                    (Transformation|SetRelativeLocation _frontcover_2 "0.200000,0.000000,0.000000" false false)))))
            (:Finished
              (switch Utilities|FlowControl|Switch|SwitchonETimelineDirection _direction
                (:Forward
                  (CallFunction|EventReset))
                (:Backward
                  (bind _result (Math|Integer|DecrementInt (Variables|Default|GetpageCount))
                    (:%20%20
                      (Variables|Default|SetpageCount (Math|Integer|Clamp(Integer) _result 0 (Variables|Default|GetMaxPages)))
                      (CallFunction|EventReset))))))))))))

(event Input|KeyboardEvents|Q
  (params (Key :type Key%20Structure))
  (bind _frontcover (Variables|Default|GetFrontCover))
  (bind _frontcover_2 (Variables|Default|GetFrontCover))
  ;[0.6201 0.42 1] [Shayenne]
  (:Pressed
    (Utilities|FlowControl|DoOnce false
      (:Completed
        (Development|PrintString "PREVIOUS PAGE")
        (if (not (== (Variables|Default|GetpageCount) 0))
          (CallFunction|PlayAudio)
          (bind (_direction _alpha) (Timeline|FlipPage ReverseFromEnd)
            (:Update
              (Transformation|SetRelativeRotation (Utilities|Select :Index (Variables|Default|GetpageCount) :Option%200 0 :Option%201 _frontcover :Option%202 (Variables|Default|GetPage_Intro) :Option%203 (Variables|Default|GetPage_One) :Option%204 (Variables|Default|GetPage_Two)) (Math|Rotator|Lerp(Rotator) "90.000000,0.000000,0.000000" "90.000000,180.000000,0.000000" _alpha) false false)
              (if (== (Utilities|Select :Index (Variables|Default|GetpageCount) :Option%200 0 :Option%201 _frontcover :Option%202 (Variables|Default|GetPage_Intro) :Option%203 (Variables|Default|GetPage_One) :Option%204 (Variables|Default|GetPage_Two)) _frontcover)
                (switch Utilities|FlowControl|Switch|SwitchonETimelineDirection _direction
                  (:Forward
                    (Transformation|SetRelativeLocation _frontcover_2 "-0.100000,0.000000,0.000000" false false))
                  (:Backward
                    (Transformation|SetRelativeLocation _frontcover_2 "0.200000,0.000000,0.000000" false false)))))
            (:Finished
              (switch Utilities|FlowControl|Switch|SwitchonETimelineDirection _direction
                (:Forward
                  (CallFunction|EventReset))
                (:Backward
                  (bind _result (Math|Integer|DecrementInt (Variables|Default|GetpageCount))
                    (:%20%20
                      (Variables|Default|SetpageCount (Math|Integer|Clamp(Integer) _result 0 (Variables|Default|GetMaxPages)))
                      (CallFunction|EventReset))))))))))))

(event Input|GamepadEvents|GamepadRightShoulder
  (params (Key :type Key%20Structure))
  (bind _frontcover (Variables|Default|GetFrontCover))
  (bind _frontcover_2 (Variables|Default|GetFrontCover))
  ;[0.6201 0.42 1] [Shayenne]
  (:Pressed
    (Utilities|FlowControl|DoOnce false
      (:Completed
        (Development|PrintString "NEXT PAGE")
        (if (== (Variables|Default|GetpageCount) (- (Variables|Default|GetMaxPages) 1))
          (CallFunction|EventFlipBack)
          (else
            (bind _result (Math|Integer|IncrementInt (Variables|Default|GetpageCount))
              (:%20%20
                (Variables|Default|SetpageCount (Math|Integer|Clamp(Integer) _result 0 (Variables|Default|GetMaxPages)))
                (CallFunction|PlayAudio)
                (bind (_direction _alpha) (Timeline|FlipPage PlayFromStart)
                  (:Update
                    (Transformation|SetRelativeRotation (Utilities|Select :Index (Variables|Default|GetpageCount) :Option%200 0 :Option%201 _frontcover :Option%202 (Variables|Default|GetPage_Intro) :Option%203 (Variables|Default|GetPage_One) :Option%204 (Variables|Default|GetPage_Two)) (Math|Rotator|Lerp(Rotator) "90.000000,0.000000,0.000000" "90.000000,180.000000,0.000000" _alpha) false false)
                    (if (== (Utilities|Select :Index (Variables|Default|GetpageCount) :Option%200 0 :Option%201 _frontcover :Option%202 (Variables|Default|GetPage_Intro) :Option%203 (Variables|Default|GetPage_One) :Option%204 (Variables|Default|GetPage_Two)) _frontcover)
                      (switch Utilities|FlowControl|Switch|SwitchonETimelineDirection _direction
                        (:Forward
                          (Transformation|SetRelativeLocation _frontcover_2 "-0.100000,0.000000,0.000000" false false))
                        (:Backward
                          (Transformation|SetRelativeLocation _frontcover_2 "0.200000,0.000000,0.000000" false false)))))
                  (:Finished
                    (switch Utilities|FlowControl|Switch|SwitchonETimelineDirection _direction
                      (:Forward
                        (CallFunction|EventReset))
                      (:Backward
                        (bind _result_2 (Math|Integer|DecrementInt (Variables|Default|GetpageCount))
                          (:%20%20
                            (Variables|Default|SetpageCount (Math|Integer|Clamp(Integer) _result_2 0 (Variables|Default|GetMaxPages)))
                            (CallFunction|EventReset)))))))))))))))

(fn ConstructionScript)