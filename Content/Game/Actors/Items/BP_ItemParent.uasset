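; BP_ItemParent is a base item Blueprint that BP_Player can pick up, hold and drop.
; Interact disables the StaticMesh's physics and collision, snaps it to the player's AttachSocket, and registers the item as HeldActor.
; Drop restores collision, calls DetachFromActor and re-enables physics, without clearing HeldActor itself.
; Pickup attaches only the mesh component, while drop detaches at actor level; the Open event is empty.
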(event EventInterfaceInteract
  (params (actor :type Actor%20Object%20Reference))
  ;[0.4604 1 0.414] Comment
  (bind _asbp_player (Utilities|Casting|CastToBP_Player actor))
  (Variables|Default|SetAs%20BP%20Player _asbp_player)
  (Physics|SetSimulatePhysics (Variables|Default|GetStaticMesh) false)
  (Transformation|AttachComponentToComponent (Variables|Default|GetStaticMesh) (Variables|/Game/Game/Player/BP_Player.BP_Player_C|Getattach_socket _asbp_player) "None" "SnapToTarget" "SnapToTarget" "KeepRelative" true)
  (Collision|SetCollisionEnabled (Variables|Default|GetStaticMesh) "NoCollision")
  (Variables|/Game/Game/Player/BP_Player.BP_Player_C|SetheldActor _asbp_player self))

(event EventInterfaceDrop
  ;[0.4604 1 0.414] Comment
  (Collision|SetCollisionEnabled (Variables|Default|GetStaticMesh) "QueryAndPhysics")
  (Transformation|DetachFromActor self "KeepWorld" "KeepWorld" "KeepWorld")
  (Physics|SetSimulatePhysics (Variables|Default|GetStaticMesh) true))

(event EventInterfaceOpen)

(fn ConstructionScript)