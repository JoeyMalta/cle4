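; Base item actor that the player can look at, pick up and drop, showing its name in an interact widget.
; Interact disables mesh physics and collision, snaps the item to BP_Player's attach socket and registers it as held; drop reverses this.
; Observe plays the widget's activate animation once, using a retriggerable delay to deactivate it when observe calls stop.
; Tick draws a debug point at the actor's location.
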(event EventBeginPlay
  (bind _aswbp_interact_item (Utilities|Casting|CastToWBP_Interact_Item (UserInterface|GetUserWidgetObject (Variables|Default|GetAC_WidgetComponent_Item))))
  (Default|UpdateItemName _aswbp_interact_item (Variables|itemSettings|GetitemName))
  (Variables|Default|SetRelative%20Location (Variables|/Script/Engine.SceneComponent|GetRelativeLocation (Variables|Default|GetScene))))

(event EventTick
  (params (DeltaSeconds :type Float%20%28single-precision%29))
  (Rendering|Debug|DrawDebugPoint (Transformation|GetActorLocation) 1e+01 "(R=0.977431,G=0.000000,B=0.000000,A=1.000000)" 1.0))

(event EventInterfaceObserve
  (Utilities|FlowControl|Sequence
    (:then_0
      (Utilities|FlowControl|DoOnce false :!label _label
        (:Completed
          (bind _aswbp_interact_item (Utilities|Casting|CastToWBP_Interact_Item (UserInterface|GetUserWidgetObject (Variables|Default|GetAC_WidgetComponent_Item))))
          (Default|ActivateAnimation _aswbp_interact_item))))
    (:then_1
      (Utilities|FlowControl|RetriggerableDelay 0.1)
      (Utilities|FlowControl|Sequence
        (:then_0
          (goto _label Reset))
        (:then_1
          (bind _aswbp_interact_item_2 (Utilities|Casting|CastToWBP_Interact_Item (UserInterface|GetUserWidgetObject (Variables|Default|GetAC_WidgetComponent_Item))))
          (Default|DeactivateAnimation _aswbp_interact_item_2))))))

(event EventInterfaceInteract
  (params (actor :type Actor%20Object%20Reference))
  (bind _staticmesh (Variables|Default|GetStaticMesh))
  (bind _asbp_player (Utilities|Casting|CastToBP_Player actor))
  (Variables|Default|SetAs%20BP%20Player _asbp_player)
  (Physics|SetSimulatePhysics (Variables|Default|GetStaticMesh) false)
  (Transformation|SetWorldLocation _staticmesh (+ (Transformation|GetActorLocation) (Variables|Default|GetRelative%20Location)) false false)
  ;[0.4604 1 0.414] Comment
  (Transformation|AttachComponentToComponent _staticmesh (Variables|Default|GetDefaultSceneRoot) "None" "SnapToTarget" "SnapToTarget" "KeepRelative" true)
  (Collision|SetCollisionEnabled (Variables|Default|GetStaticMesh) "NoCollision")
  (Transformation|AttachComponentToComponent (Variables|/Game/Game/Player/BP_Player.BP_Player_C|Getattach_socket _asbp_player) "None" "SnapToTarget" "SnapToTarget" "KeepRelative" true)
  (Variables|/Game/Game/Player/BP_Player.BP_Player_C|SetBP_HeldActor _asbp_player self))

(event EventInterfaceDrop
  ;[0.4604 1 0.414] Comment
  (Collision|SetCollisionEnabled (Variables|Default|GetStaticMesh) "QueryAndPhysics")
  (Transformation|DetachFromActor self "KeepWorld" "KeepWorld" "KeepRelative")
  (Physics|SetSimulatePhysics (Variables|Default|GetStaticMesh) true)
  (bind _as_bp_player (Variables|Default|GetAs%20BP%20Player)
    (:then
      (Variables|/Game/Game/Player/BP_Player.BP_Player_C|SetBP_HeldActor _as_bp_player 0))
    (:else)))

(fn ConstructionScript)