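; Delivery truck actor that waits to be loaded with every cardboard box in the level, then drives off.
; An external call to CheckBoxAmount stores the box total, which Tick compares against boxes overlapping its trigger.
; On a match it fires once: after a short delay it attaches the boxes, honks and hands itself to the "spline02" BP_TruckSpline to drive to delivery.
; It then completes the load-truck task for the current round.
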(event Custom|event_CheckBoxAmount
  ;[0.6201 0.42 1] [shayenne] hier komt een custom event die checked hoeveel dozen er in het level bestaan op dat moment.
  (bind _outactors (Actor|GetAllActorsOfClass "/Game/Game/Actors/Cardboard/BP_CardboardBox.BP_CardboardBox_C"))
  (Variables|Default|SetTotalBoxes (Utilities|Array|Length _outactors)))

(event Custom|event_CompleteLoadTruck
  ;[0.6201 0.42 1] [shayenne]
  (switch Utilities|FlowControl|Switch|SwitchonE_ScenarioOne_Round (CallFunction|GetCurrentRound)
    (:NewEnumerator0
      (Utilities|FlowControl|DoOnce false
        (:Completed
          (Default|CompleteTask (CallFunction|GetTasklist) "NewEnumerator2"))))
    (:NewEnumerator1
      (Utilities|FlowControl|DoOnce false
        (:Completed
          (Default|CompleteTask (CallFunction|GetTasklist) "NewEnumerator2"))))
    (:NewEnumerator2
      (Utilities|FlowControl|DoOnce false
        (:Completed
          (Default|CompleteTask (CallFunction|GetTasklist) "NewEnumerator2"))))))

(event EventBeginPlay
  (Utilities|FlowControl|Delay 8.0)
  (Audio|Components|Audio|Play (Variables|Default|GetHonk) 0.0))

(event EventTick
  (params (DeltaSeconds :type Float%20%28single-precision%29))
  (bind _honk (Variables|Default|GetHonk))
  ;[0.6201 0.42 1] [shayenne] hier komt een custom event die checked hoeveel dozen er in het level bestaan op dat moment.
  (if (> (Variables|Default|GetTotalBoxes) 0)
    (bind _output_get (Variables|Default|SetOverlapping%20Actors (Collision|GetOverlappingActors (Variables|Default|GetBox) "/Game/Game/Actors/Cardboard/BP_CardboardBox.BP_CardboardBox_C" :!class /Script/Engine.PrimitiveComponent)))
    (if (== (Variables|Default|GetTotalBoxes) (Utilities|Array|Length _output_get))
      (Utilities|FlowControl|DoOnce false
        (:Completed
          (Development|PrintString "Me is leaving" true true "(R=1.000000,G=0.873810,B=0.016375,A=1.000000)" 33.0)
          (Utilities|FlowControl|Delay 2.0)
          (for _array_element (Variables|Default|GetOverlapping%20Actors)
            (bind _asbp_cardboard_box (Utilities|Casting|CastToBP_CardboardBox _array_element))
            (Transformation|AttachActorToActor _array_element self "None" "SnapToTarget" "KeepRelative" "KeepRelative" true)
            (Transformation|AttachComponentToComponent (Variables|/Game/Game/Player/PickupSystem/BP_Pickup_Parent.BP_Pickup_Parent_C|GetStaticMesh _asbp_cardboard_box) (Variables|Default|GetTruckBody) "None" "KeepWorld" "KeepWorld" "KeepWorld" true))
          (Audio|Components|Audio|SetSound _honk "/Game/Game/Actors/Truck/SFX/SFX_TruckLeaving.SFX_TruckLeaving")
          (Audio|Components|Audio|Play _honk 0.0)
          (bind _outactors (Actor|GetAllActorswithTag "spline02"))
          (bind _asbp_truck_spline (Utilities|Casting|CastToBP_TruckSpline (Utilities|Array|Get(acopy) _outactors)))
          (Variables|/Game/Game/Actors/Truck/BP_TruckSpline.BP_TruckSpline_C|SetSpawnedTruck _asbp_truck_spline self)
          (Default|EventDrivetoDeliveryPoint _asbp_truck_spline)
          (CallFunction|EventCompleteLoadTruck))))))

(fn ConstructionScript)

(fn FunctionCalculateSomething)