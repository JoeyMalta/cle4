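; BP_TruckSpline is a spline path segment that drives a BP_Truck toward a delivery point.
; A timeline slowed by play rate moves and rotates the truck along the spline.
; On finish it hands the truck to the next linked spline, chaining segments, or prints a placeholder for an end-of-score event.
; A flag gates truck spawning, but the spawn-and-drive startup logic is disconnected and BeginPlay is empty.
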(event Custom|event_NextSpline
  (params (NewParam :type BP%20Truck%20Object%20Reference))
  (Variables|Default|SetSpawnedTruck NewParam)
  (CallFunction|EventDrivetoDeliveryPoint))

(event Custom|Event_SpawnTruck
  (if (Variables|Default|GetisAllowedToSpawnTruck)
    (bind _returnvalue (Game|SpawnActorfromClass "/Game/Game/Actors/Truck/BP_Truck.BP_Truck_C" (Math|Transform|MakeTransform (Transformation|GetActorLocation) (Transformation|GetActorRotation) "1.000000,1.000000,1.000000") "AlwaysSpawn" "MultiplyWithRoot" 0 0))
    (Variables|Default|SetSpawnedTruck _returnvalue)))

(event Custom|Event_DriveToDeliveryPoint
  (bind _spline (Variables|Default|GetSpline))
  (Components|Timeline|SetPlayRate (Variables|Default|GetT_TruckToPoint) (/ 1.0 1e+01))
  (bind _trucktodelivery (Timeline|T_TruckToPoint Play)
    (:Update
      (Development|PrintString (Utilities|String|ToString(Float) _trucktodelivery))
      (Transformation|SetActorLocation (Variables|Default|GetSpawnedTruck) (Spline|GetLocationatDistanceAlongSpline _spline (Math|Float|Lerp 0.0 (Spline|GetSplineLength (Variables|Default|GetSpline)) (Math|Float|Clamp(Float) _trucktodelivery)) "World") false false)
      (Transformation|SetActorRotation (Variables|Default|GetSpawnedTruck) (Spline|GetRotationatDistanceAlongSpline _spline (Math|Float|Lerp 0.0 (Spline|GetSplineLength (Variables|Default|GetSpline)) (Math|Float|Clamp(Float) _trucktodelivery)) "World")))
    (:Finished
      (bind _bp_nexttruckspline (Variables|Default|GetBP_NextTruckSpline)
        (:then
          (CallFunction|EventNextSpline _bp_nexttruckspline (Variables|Default|GetSpawnedTruck)))
        (:else
          (Development|PrintString "maak voor mij een evetn zodat ik die kan gebruiken voor score einde widget something yay"))))))

(event EventBeginPlay)

(fn ConstructionScript)