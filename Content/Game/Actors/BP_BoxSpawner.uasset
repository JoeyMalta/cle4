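; BP_BoxSpawner is an actor that spawns a batch of cardboard boxes when play begins.
; A custom ForLoopDelay macro runs a fixed count with a short delay between iterations, spreading the spawns over time.
; Each iteration spawns a BP_CardboardBox at a random point inside the Box component's bounds and calls InitBox on it.
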(event EventBeginPlay
  (bind _box (Variables|Default|GetBox))
  (Utilities|ForLoopDelay 0 9 0.2
    (:LoopBody
      (bind _returnvalue (Game|SpawnActorfromClass "/Game/Game/Actors/BP_CardboardBox.BP_CardboardBox_C" (Math|Transform|MakeTransform (Math|Random|RandomPointinBoundingBox (Transformation|GetWorldLocation _box) (Variables|/Script/Engine.BoxComponent|GetBoxExtent _box)) "0, 0, 0" "1.000000,1.000000,1.000000") "Undefined" "MultiplyWithRoot" 0 0))
      (Default|InitBox _returnvalue))))

(fn ConstructionScript)