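; Conveyor belt socket that holds one item and pulls a replacement from linked sockets when freed, cascading items along.
; Occupy binds the item's pickup event and slides it to the socket with a timeline lerp.
; On pickup, socket 0 refills from the first occupied socket in ID0Array; Unoccupy lets sockets 1 and 2 do likewise.
; A text render shows occupancy in red or green.
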(event Custom|event_MoveItem
  (Variables|Default|SetActorLocation (Transformation|GetActorLocation (Variables|Default|GetActor)))
  (Components|Timeline|SetPlayRate (Variables|Default|GetSmoothLerp) (/ 1.0 2.0))
  (bind _alpha (Timeline|SmoothLerp PlayFromStart)
    (:Update
      (Transformation|SetActorLocation (Variables|Default|GetActor) (Math|Vector|Lerp(Vector) (Variables|Default|GetActorLocation) (Transformation|GetActorLocation) _alpha) false false))))

(event Custom|assignActor
  (params (NewParam :type BP%20Item%20Parent%20Object%20Reference))
  (EventDispatchers|AssignEventonPickedUp NewParam (delegate Custom|event_OnPickedUp_Event))
  (CallFunction|EventMoveItem))

(event Custom|event_OnPickedUp_Event
  (params (ItemID :type Integer))
  (Audio|Components|Audio|Stop (Variables|Default|GetSmoothLerp))
  (CallFunction|Unoccupy)
  (switch int (Variables|Default|GetSocketID)
    (:0
      (bind _array_element (CallFunction|FindPotentialCandidate))
      (if (Utilities|IsValid _array_element)
        (CallFunction|Occupy (Variables|BP_ConveyerSocket_C|GetActor _array_element))
        (CallFunction|Unoccupy _array_element)))))

(event Custom|event_CheckUnoccupiedState
  (switch int (Variables|Default|GetSocketID)
    (:1
      (bind _array_element (CallFunction|FindPotentialCandidate))
      (Utilities|IsValid _array_element
        (:Is%20Valid
          (CallFunction|Occupy (Variables|BP_ConveyerSocket_C|GetActor _array_element))
          (CallFunction|Unoccupy _array_element))))
    (:2
      (bind _array_element_2 (CallFunction|FindPotentialCandidate))
      (Utilities|IsValid _array_element_2
        (:Is%20Valid
          (CallFunction|Occupy (Variables|BP_ConveyerSocket_C|GetActor _array_element_2))
          (CallFunction|Unoccupy _array_element_2))))))

(fn ConstructionScript)

(fn Occupy
  (params (Actor :type BP%20Item%20Parent%20Object%20Reference))
  (bind _textrender (Variables|Default|GetTextRender))
  (bind _output_get (Variables|Default|SetActor Actor))
  (CallFunction|AssignActor _output_get)
  (Variables|Default|SetisOccupied true)
  (Rendering|Components|TextRender|SetText _textrender (Utilities|Text|FormatText "Occupied"))
  (Rendering|Components|TextRender|SetTextRenderColor _textrender (Math|Conversions|ToColor(LinearColor) "(R=0.977431,G=0.000000,B=0.000000,A=1.000000)")))

(fn Unoccupy
  (bind _textrender (Variables|Default|GetTextRender))
  (Rendering|Components|TextRender|SetText _textrender (Utilities|Text|FormatText "Unoccupied"))
  (Rendering|Components|TextRender|SetTextRenderColor _textrender (Math|Conversions|ToColor(LinearColor) "(R=0.435954,G=0.979167,B=0.389286,A=1.000000)"))
  (Variables|Default|SetActor 0)
  (Variables|Default|SetisOccupied false)
  (CallFunction|EventCheckUnoccupiedState))

(fn FindPotentialCandidate
  (for _array_element (Variables|Default|GetID0_Array)
    (if (Variables|BP_ConveyerSocket_C|GetisOccupied _array_element)
      (return _array_element))))