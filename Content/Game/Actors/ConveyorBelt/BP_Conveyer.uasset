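; BP_Conveyer is a conveyor belt actor meant to carry items along a spline.
; On BeginPlay it calls SpawnItemOnSpline, which spawns an actor at the belt's own location, with no spline logic yet.
; UpdateSlot takes AvailableSlots entries above a given index, lowers each item's ItemID to one below its key and collects them in TempList under the new keys.
; TempList is not written back to AvailableSlots here.
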(event Custom|SpawnItemOnSpline
  ;[0.15 0.15 0.15 0.5] Comment
  (Game|SpawnActorfromClass "/Game/Game/Actors/Items/BP_Medicin.BP_Medicin_C" (Math|Transform|MakeTransform (Transformation|GetActorLocation) "0, 0, 0" "1.000000,1.000000,1.000000") "AlwaysSpawn" "MultiplyWithRoot" 0 0 0))

(event EventBeginPlay
  ;[0.15 0.15 0.15 0.5] Comment
  (CallFunction|SpawnItemonSpline))

(fn ConstructionScript)

(fn UpdateSlot
  (params (NewParam :type Integer))
  (Utilities|Map|Clear (Variables|Default|GetTempList))
  (bind (_keypin _valuepin) (Utilities|Map|ForEachLoop(Map) (Variables|Default|GetAvailableSlots))
    (:then
      (if (> _keypin NewParam)
        (bind _asbp_item_parent (Utilities|Casting|CastToBP_ItemParent _valuepin))
        (Variables|/Game/Game/Actors/Items/Core/BP_ItemParent.BP_ItemParent_C|SetitemID _asbp_item_parent (- _keypin 1))
        (Utilities|Map|Add (Variables|Default|GetTempList) (- _keypin 1) _valuepin)))
    (:CompletedPin
      (return))))