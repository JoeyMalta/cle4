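; BP_HingeDoor is a hinged door actor in the conveyor belt set that bursts open to kick cardboard boxes into the level.
; A spawn request stores the amount and plays a hinge Timeline, whose forward finish triggers the throw and BP_Leg's kick.
; A delayed-loop macro launches randomly chosen boxes along the Arrow with impulse and sound.
; The door then reverses shut, creating a tasklist task in round one.
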(event Custom|Open%20Door
  (Audio|PlaySoundatLocation "/Game/Game/Actors/ConveyorBelt/Door/SFX/SFX_OpenDoor.SFX_OpenDoor" (Transformation|GetActorLocation) "0, 0, 0" 1.0 1.5 0.0 0 0 0 0)
  (bind (_direction _newtrack1 _openhingeddoor _opendoorhinge) (Timeline|Timeline PlayFromStart)
    (:Update
      (Transformation|SetRelativeRotation (Variables|Default|GetDoor) (Math|Rotator|MakeRotator 0.0 0.0 _opendoorhinge) false false))
    (:Finished
      (switch Utilities|FlowControl|Switch|SwitchonETimelineDirection _direction
        (:Forward
          (CallFunction|EventThrowBox))
        (:Backward
          (Audio|PlaySoundatLocation "/Game/Game/Actors/ConveyorBelt/Door/SFX/SFX_CloseDoor.SFX_CloseDoor" (Transformation|GetActorLocation) "0, 0, 0" 1.0 1.5 0.0 "/Game/Game/Actors/ConveyorBelt/Door/SoundDistance.SoundDistance" 0 0 0))))))

(event Custom|CLoseDoor
  (bind (_direction _newtrack1 _openhingeddoor _opendoorhinge) (Timeline|Timeline ReverseFromEnd)
    (:Update
      (Transformation|SetRelativeRotation (Variables|Default|GetDoor) (Math|Rotator|MakeRotator 0.0 0.0 _opendoorhinge) false false))
    (:Finished
      (switch Utilities|FlowControl|Switch|SwitchonETimelineDirection _direction
        (:Forward
          (CallFunction|EventThrowBox))
        (:Backward
          (Audio|PlaySoundatLocation "/Game/Game/Actors/ConveyorBelt/Door/SFX/SFX_CloseDoor.SFX_CloseDoor" (Transformation|GetActorLocation) "0, 0, 0" 1.0 1.5 0.0 "/Game/Game/Actors/ConveyorBelt/Door/SoundDistance.SoundDistance" 0 0 0))))))

(event Custom|event_SpawnBox
  (params (amount :type Integer))
  (Variables|Default|SetAmount amount)
  (CallFunction|OpenDoor))

(event Custom|event_ThrowBox
  (bind _availableboxes (Variables|Default|GetAvailableBoxes))
  (Utilities|FlowControl|Sequence
    (:then_0
      (Utilities|Array|Shuffle (Variables|Default|GetAvailableBoxes))
      (Utilities|ForLoopDelay 0 (Variables|Default|GetAmount) 0.4
        (:LoopBody
          (bind _returnvalue (Game|SpawnActorfromClass "/Game/Game/Actors/Cardboard/BP_CardboardBox.BP_CardboardBox_C" (Transformation|GetWorldTransform (Variables|Default|GetArrow)) "AlwaysSpawn" "MultiplyWithRoot" 0 (Utilities|Array|Get(acopy) _availableboxes (Math|Random|RandomIntegerinRange 0 (- (Utilities|Array|Length _availableboxes) 1))) 0))
          (Default|InterfaceDrop _returnvalue false)
          (Physics|AddImpulse (Variables|/Game/Game/Player/PickupSystem/BP_Pickup_Parent.BP_Pickup_Parent_C|GetStaticMesh _returnvalue) (* (Math|Vector|GetForwardVector (Variables|Default|GetArrow)) 1e+03) "None" true)
          (Audio|PlaySoundatLocation "/Game/Game/Actors/Cardboard/SFX/SFX_CardboardBox_Kicked.SFX_CardboardBox_Kicked" (Transformation|GetActorLocation _returnvalue) "0, 0, 0" 1.0 (Math|Random|RandomFloatinRange 0.8 1.0) 0.0 "/Game/Game/Actors/ConveyorBelt/Door/SoundDistance.SoundDistance" 0 0 0))
        (:Completed
          (Utilities|FlowControl|Delay 0.5)
          (CallFunction|CLoseDoor)
          (switch Utilities|FlowControl|Switch|SwitchonE_ScenarioOne_Round (CallFunction|GetCurrentRound)
            (:NewEnumerator0
              (Default|CreateTask (CallFunction|GetTasklist) "NewEnumerator0"))))))
    (:then_1
      (bind _returnvalue_2 (Actor|GetActorOfClass "/Game/Assets/Anna/BP_Leg.BP_Leg_C"))
      (Default|Kick _returnvalue_2))))

(event EventBeginPlay
  (Components|Timeline|SetPlayRate (Variables|Default|GetTimeline) (/ 1.0 0.2)))

(fn ConstructionScript)