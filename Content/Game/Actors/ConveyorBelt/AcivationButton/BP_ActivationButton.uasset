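; Interactable activation button that starts the conveyor belt sequence and advances the tasklist.
; Observing it animates its widget; interacting runs once per round branch, completing the activation task and creating that round's follow-up tasks after a delay.
; Activation updates the widget text, triggers the alert light, then opens the garage door after a delay.
; The door's finished event triggers item spawning on the conveyor's spline.
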(event Custom|event_Finished_Event
  (bind _returnvalue (Actor|GetActorOfClass "/Game/Game/Actors/ConveyorBelt/BP_Conveyer.BP_Conveyer_C"))
  (Default|SpawnItemonSpline _returnvalue))

(event Custom|event_ActivateButtonLogic
  (bind _aswbp_interact_conveyor_button (Utilities|Casting|CastToWBP_Interact_ConveyorButton (UserInterface|GetUserWidgetObject (Variables|Default|GetAC_ActivationButton))))
  (Default|UpdateText _aswbp_interact_conveyor_button "Activated")
  (bind _returnvalue (Actor|GetActorOfClass "/Game/Game/Actors/ConveyorBelt/BP_AlertLight.BP_AlertLight_C"))
  (Default|ActivateAlarm _returnvalue)
  (Utilities|FlowControl|Delay 3.0)
  (bind _returnvalue_2 (Actor|GetActorOfClass "/Game/Assets/Anna/BP_GarageDoor.BP_GarageDoor_C"))
  (Default|OpenDoor _returnvalue_2)
  (EventDispatchers|AssignEventFinished _returnvalue_2 (delegate Custom|event_Finished_Event)))

(event EventInterfaceObserve
  (params (OwningPlayer :type Actor%20Object%20Reference) (isHoldingObject :type Boolean) (hitResult :type Hit%20Result%20Structure))
  (bind _aswbp_interact_conveyor_button (Utilities|Casting|CastToWBP_Interact_ConveyorButton (UserInterface|GetUserWidgetObject (Variables|Default|GetAC_ActivationButton))))
  (Default|ActivateAnimation _aswbp_interact_conveyor_button))

(event EventInterfaceInteract
  (params (actor :type Actor%20Object%20Reference) (isHoldingObject :type Boolean) (hitResult :type Hit%20Result%20Structure))
  (switch Utilities|FlowControl|Switch|SwitchonE_ScenarioOne_Round (CallFunction|GetCurrentRound)
    (:NewEnumerator0
      (Utilities|FlowControl|DoOnce false
        (:Completed
          (CallFunction|EventActivateButtonLogic)
          (Default|CompleteTask (CallFunction|GetTasklist) "NewEnumerator5")
          (Utilities|FlowControl|Delay 2.0)
          (Default|CreateTask (CallFunction|GetTasklist) "NewEnumerator1"))))
    (:NewEnumerator1
      ;[0.6201 0.42 1] Comment
      (Utilities|FlowControl|DoOnce false
        (:Completed
          (CallFunction|EventActivateButtonLogic)
          (Default|CompleteTask (CallFunction|GetTasklist) "NewEnumerator5")
          (Utilities|FlowControl|Delay 2.0)
          (Default|CreateTask (CallFunction|GetTasklist) "NewEnumerator1")
          (Default|CreateTask (CallFunction|GetTasklist) "NewEnumerator3"))))
    (:NewEnumerator2
      (Utilities|FlowControl|DoOnce false
        (:Completed
          (CallFunction|EventActivateButtonLogic)
          (Default|CompleteTask (CallFunction|GetTasklist) "NewEnumerator5")
          (Utilities|FlowControl|Delay 2.0)
          (Default|CreateTask (CallFunction|GetTasklist) "NewEnumerator1")
          (Default|CreateTask (CallFunction|GetTasklist) "NewEnumerator3")
          (Default|CreateTask (CallFunction|GetTasklist) "NewEnumerator4"))))))

(fn ConstructionScript)