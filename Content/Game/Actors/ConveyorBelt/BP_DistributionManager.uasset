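; BP_DistributionManager runs the rounds of a conveyor-belt box distribution sequence.
; ResetRound fades the screen, resets the conveyor, alert light and garage door, returns the player to PlayerStart, clears the fine widget, then starts distribution.
; StartDistribution branches on the current round, using DoOnce to tell the hinge door to spawn that round's box.
; Round one also creates the HUD task list; a fine-widget creation call is left unconnected.
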(event Custom|startDistribution
  (switch Utilities|FlowControl|Switch|SwitchonE_ScenarioOne_Round (CallFunction|GetCurrentRound)
    (:NewEnumerator0
      (Utilities|FlowControl|DoOnce false
        (:Completed
          (bind _ashud_player_interface (Utilities|Casting|CastToHUD_PlayerInterface (HUD|GetHUD (Game|GetPlayerController 0))))
          (Default|EventCreateTaskList _ashud_player_interface)
          (bind _returnvalue (Actor|GetActorOfClass "/Game/Game/Actors/ConveyorBelt/Door/BP_HingeDoor.BP_HingeDoor_C"))
          (Default|EventSpawnBox _returnvalue))))
    (:NewEnumerator1
      (Utilities|FlowControl|DoOnce false
        (:Completed
          (bind _returnvalue_2 (Actor|GetActorOfClass "/Game/Game/Actors/ConveyorBelt/Door/BP_HingeDoor.BP_HingeDoor_C"))
          (Default|EventSpawnBox _returnvalue_2 1))))))

(event Custom|ResetRound
  (bind _ashud_player_interface (Utilities|Casting|CastToHUD_PlayerInterface (HUD|GetHUD (Game|GetPlayerController 0))))
  (Default|TransitionFadetoBlack _ashud_player_interface)
  (Utilities|FlowControl|Delay 2.0)
  (bind _returnvalue (Actor|GetActorOfClass "/Game/Game/Actors/ConveyorBelt/BP_Conveyer.BP_Conveyer_C"))
  (Default|ResetConveyor _returnvalue)
  (bind _returnvalue_2 (Actor|GetActorOfClass "/Game/Game/Actors/ConveyorBelt/BP_AlertLight.BP_AlertLight_C"))
  (Default|DeactivateAlarm _returnvalue_2)
  (bind _returnvalue_3 (Actor|GetActorOfClass "/Game/Assets/Anna/BP_GarageDoor.BP_GarageDoor_C"))
  (Default|CLoseDoor _returnvalue_3)
  (bind _returnvalue_4 (Actor|GetActorOfClass "/Script/Engine.PlayerStart"))
  (Transformation|SetActorTransform (Game|GetPlayerCharacter 0) (Transformation|GetActorTransform _returnvalue_4))
  (Utilities|FlowControl|Delay 2.0)
  (bind _ashud_player_interface_2 (Utilities|Casting|CastToHUD_PlayerInterface (HUD|GetHUD (Game|GetPlayerController 0))))
  (Default|TransitionFadetoBack _ashud_player_interface_2)
  (Utilities|FlowControl|Delay 2.0)
  (Widget|RemovefromParent (Variables|/Game/Game/Player/HUD_PlayerInterface.HUD_PlayerInterface_C|GetWBP_FinedWidget _ashud_player_interface_2))
  (CallFunction|StartDistribution))

(event EventBeginPlay)

(fn ConstructionScript)