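; BP_AlertLight is an alarm light actor in the conveyor belt set, with two spotlights, an audio component and a spinning Arrow component.
; activateAlarm enables tick, starts the sound and lights both spotlights, while deactivateAlarm reverses all three.
; Tick rotates the Arrow by a fixed local step each frame without delta time, so the spin speed depends on frame rate.
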(event Custom|activateAlarm
  (Actor|Tick|SetActorTickEnabled true)
  (Audio|Components|Audio|Play (Variables|Default|GetAudio) 0.0)
  (Rendering|Components|Light|SetIntensity (Variables|Default|GetSpotLight1) 2.5e+03))

(event Custom|deactivateAlarm
  (Actor|Tick|SetActorTickEnabled false)
  (Audio|Components|Audio|Stop (Variables|Default|GetAudio))
  (Rendering|Components|Light|SetIntensity (Variables|Default|GetSpotLight1) 0.0))

(event EventTick
  (params (DeltaSeconds :type Float%20%28single-precision%29))
  (Transformation|AddLocalRotation (Variables|Default|GetArrow) "0.000000,0.000000,5.000000" false false))

(fn ConstructionScript)