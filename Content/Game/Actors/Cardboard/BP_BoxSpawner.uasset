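; Box spawner actor meant to scatter cardboard boxes, each tied to a country row in DT_CardboardData.
; A delayed-loop macro, ForLoopDelay, spawns BP_CardboardBox at random points inside a Box component, passes the row handle, then initializes it.
; The spawn chain is disconnected from BeginPlay, so it never runs.
; Its loop makes ten passes, but the index-based Select maps only five countries.
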(event EventBeginPlay
  ;[0.4508 0.9792 0.4054] [Joey] Spawnt meerdere kartonnen dozen op willekeurige locaties en koppelt aan elke doos een land uit de Data Table.
)

(fn ConstructionScript)