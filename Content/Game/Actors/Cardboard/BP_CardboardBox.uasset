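; Interactable cardboard box that the player can pick up, drop, open or close, and fill with held items.
; A data table row sets its shade color via dynamic material, country flag, weight label and panel flag.
; Interacting empty-handed attaches the box to the player; with a held item, it snaps that item into one of four sockets if open, otherwise plays a widget error.
; Initialization enables physics and plays a bounce-scale timeline.
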(event Custom|event_InitializeBox
  ;[0.4508 0.9792 0.4054] [Joey] Initialiseert de doos door physics in te schakelen en een bounce-animatie af te spelen.
  (Physics|SetSimulatePhysics (Variables|Default|GetStaticMesh) true)
  (Components|Timeline|SetNewTime (Variables|Default|GetBounce) (/ 1.0 0.2))
  (bind _scale (Timeline|Bounce PlayFromStart)
    (:Update
      (Transformation|SetRelativeScale3D (Variables|Default|GetStaticMesh) _scale))))

(event Custom|event_BoxError
  ;[0.15 0.15 0.15 0.5] Comment
  (bind _aswbp_interact_panel (Utilities|Casting|CastToWBP_InteractPanel (UserInterface|GetUserWidgetObject (Variables|Default|GetAC_WidgetComponent))))
  (Default|ErrorOpenBoxAnimation _aswbp_interact_panel))

(event Custom|event_PickUp
  ;[0.15 0.15 0.15 0.5] Comment
  (bind _bp_playercharacter (Variables|Default|GetBP_PlayerCharacter)
    (:then
      (Physics|SetSimulatePhysics (Variables|Default|GetStaticMesh) false)
      (Transformation|AttachComponentToComponent (Variables|Default|GetStaticMesh) (Variables|/Game/Game/Player/BP_Player.BP_Player_C|Getattach_socket _bp_playercharacter) "None" "SnapToTarget" "SnapToTarget" "KeepRelative" true)
      (Collision|SetCollisionEnabled (Variables|Default|GetStaticMesh) "NoCollision")
      (bind _bp_playercharacter_2 (Variables|Default|GetBP_PlayerCharacter)
        (:then
          (Variables|/Game/Game/Player/BP_Player.BP_Player_C|SetBP_HeldActor _bp_playercharacter_2 self))
        (:else)))
    (:else)))

(event EventInterfaceOpen
  (bind _staticmesh (Variables|Default|GetStaticMesh))
  ;[0.436 0.9792 0.3893] [Joey] Wisselt tussen de open en gesloten staat van het object en werkt de interactietekst bij.
  (Utilities|FlowControl|FlipFlop
    (:A
      (Components|StaticMesh|SetStaticMesh _staticmesh "/Game/Assets/Mega_Survival_Tools/Models/SM_Cardboard_Box_01_Open.SM_Cardboard_Box_01_Open")
      (bind _aswbp_interact_panel (Utilities|Casting|CastToWBP_InteractPanel (UserInterface|GetUserWidgetObject (Variables|Default|GetAC_WidgetComponent))))
      (Default|UpdateOpenText _aswbp_interact_panel "Close Object")
      (Variables|Default|SetisOpen true))
    (:B
      (Components|StaticMesh|SetStaticMesh _staticmesh "/Game/Assets/Mega_Survival_Tools/Models/SM_Cardboard_Box_01_Closed.SM_Cardboard_Box_01_Closed")
      (bind _aswbp_interact_panel_2 (Utilities|Casting|CastToWBP_InteractPanel (UserInterface|GetUserWidgetObject (Variables|Default|GetAC_WidgetComponent))))
      (Default|UpdateOpenText _aswbp_interact_panel_2 "Open Object")
      (Variables|Default|SetisOpen false))))

(event EventBeginPlay
  (bind _f_cardboarddata (Variables|Default|GetF_CardboardData))
  (bind (_datatable _rowname) (Utilities|Struct|BreakDataTableRowHandle _f_cardboarddata))
  ;[0.4508 0.9792 0.4054] [Joey] Haalt de vlag uit de geselecteerde Data Table Row en toont deze in het interactiepaneel.
  (bind _returnvalue (Utilities|GetDataTableRow _datatable _rowname)
    (:then
      (bind _aswbp_interact_panel (Utilities|Casting|CastToWBP_InteractPanel (UserInterface|GetUserWidgetObject (Variables|Default|GetAC_WidgetComponent))))
      (Default|UpdateFlag _aswbp_interact_panel (Utilities|Struct|BreakF_CardboardData _returnvalue)))))

(event EventInterfaceObserve
  ;[0.436 0.9792 0.3893] Comment
  (bind _aswbp_interact_panel (Utilities|Casting|CastToWBP_InteractPanel (UserInterface|GetUserWidgetObject (Variables|Default|GetAC_WidgetComponent))))
  (Default|UpdateWidget _aswbp_interact_panel))

(event EventInterfaceInteract
  (params (actor :type Actor%20Object%20Reference))
  ;[0.4508 0.9792 0.4054] [Joey] Pakt een interactable actor op en koppelt deze aan de speler.
  (bind _asbp_player (Utilities|Casting|CastToBP_Player actor))
  (bind _output_get (Variables|Default|SetBP_PlayerCharacter _asbp_player))
  (bind _bp_heldactor (Variables|/Game/Game/Player/BP_Player.BP_Player_C|GetBP_HeldActor _output_get)
    (:then
      (Utilities|Casting|CastToBP_ItemParent _bp_heldactor)
      (if (Variables|Default|GetisOpen)
        (bind _array_element (CallFunction|GetAvailableSlot))
        (Development|PrintString (Utilities|GetDisplayName _array_element))
        (Transformation|AttachComponentToComponent (Variables|/Game/Game/Player/BP_Player.BP_Player_C|GetBP_HeldActor (Variables|Default|GetBP_PlayerCharacter)) _array_element "None" "SnapToTarget" "SnapToTarget" "SnapToTarget" true)
        (Variables|/Game/Game/Player/BP_Player.BP_Player_C|SetBP_HeldActor (Variables|Default|GetBP_PlayerCharacter) 0)
        (else
          (CallFunction|EventBoxError))))
    (:else
      (CallFunction|EventPickUp))))

(event EventInterfaceDrop
  ;[0.4508 0.9792 0.4054] [Joey] Dropt het huidige object door collision en physics opnieuw in te schakelen.
  (Collision|SetCollisionEnabled (Variables|Default|GetStaticMesh) "QueryAndPhysics")
  (Transformation|DetachFromActor self "KeepWorld" "KeepWorld" "KeepWorld")
  (Physics|SetSimulatePhysics (Variables|Default|GetStaticMesh) true)
  (bind _bp_playercharacter (Variables|Default|GetBP_PlayerCharacter)
    (:then
      (Variables|/Game/Game/Player/BP_Player.BP_Player_C|SetBP_HeldActor _bp_playercharacter 0))
    (:else)))

(fn ConstructionScript
  (bind _f_cardboarddata (Variables|Default|GetF_CardboardData))
  (bind (_datatable _rowname) (Utilities|Struct|BreakDataTableRowHandle _f_cardboarddata))
  (|CallParentFunction)
  (bind _returnvalue (Rendering|Material|CreateDynamicMaterialInstance "/Game/Assets/Mega_Survival_Tools/Materials/MI_MainMaterial.MI_MainMaterial" "None" "None" :!class /Script/Engine.KismetMaterialLibrary))
  (LocalVariables|SetdynamicMaterial _returnvalue)
  (bind _staticmesh (Variables|Default|GetStaticMesh)
    (:then
      (Rendering|Material|SetMaterial _staticmesh 0 (LocalVariables|GetdynamicMaterial))
      (bind _returnvalue_2 (Utilities|GetDataTableRow _datatable _rowname)
        (:then
          (bind _dynamicmaterial (LocalVariables|GetdynamicMaterial)
            (:then
              (Rendering|Material|SetVectorParameterValue _dynamicmaterial "ShadeColor" (Utilities|Select :Index (.BoxColor (Utilities|Struct|BreakF_CardboardData _returnvalue_2)) :NewEnumerator0 "(R=1.000000,G=0.925847,B=0.190564,A=1.000000)" :NewEnumerator1 "(R=0.240886,G=1.000000,B=0.153094,A=1.000000)" :NewEnumerator2 "(R=1.000000,G=0.021885,B=0.005120,A=1.000000)" :NewEnumerator3 "(R=0.190713,G=0.396075,B=1.000000,A=1.000000)" :NewEnumerator4 "(R=1.000000,G=0.166538,B=0.964498,A=1.000000)") :!class /Script/Engine.MaterialInstanceDynamic)
              (Rendering|Material|SetMaterial (Variables|Default|GetCountryFlag) 0 (.material (Utilities|Struct|BreakF_CardboardData _returnvalue_2)))
              (Rendering|Components|TextRender|SetText (Variables|Default|GetKilogramsText) (Utilities|Text|FormatText "{Kilo}KG" (.WeightKG (Utilities|Struct|BreakF_CardboardData _returnvalue_2)))))
            (:else)))))
    (:else)))

(fn GetAvailableSlot
  (bind _itemsocket_01 (Variables|Default|GetItemSocket_01))
  (for (_array_element _array_index) (Variables|Default|GetAvailableSpots)
    (Utilities|IsValid _array_element
      (:Is%20Not%20Valid
        (Utilities|Array|SetArrayElem (Variables|Default|GetAvailableSpots) _array_index (Variables|/Game/Game/Player/BP_Player.BP_Player_C|GetBP_HeldActor (Variables|Default|GetBP_PlayerCharacter)))
        (return (Utilities|Array|Get(acopy) (Utilities|Array|MakeArray _itemsocket_01 (Variables|Default|GetItemSocket_02) (Variables|Default|GetItemSocket_03) (Variables|Default|GetItemSocket_04)) _array_index)))))
  (return _itemsocket_01))