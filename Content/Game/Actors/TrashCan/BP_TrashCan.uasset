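; Trash can actor that lets the player dispose of the actor they are holding by interacting with it.
; Interact destroys the player's held actor, while observe triggers the animation on the trash bin's interact widget.
; A separate bounce event, not called within this graph, plays a trash sound at the can and scales its mesh through a short timeline.
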(event Custom|even_PlayBounceAnim
  (Components|Timeline|SetPlayRate (Variables|Default|GetScaling) (/ 1.0 0.25))
  (Audio|PlaySoundatLocation "/Game/Game/Actors/TrashCan/SFX/SFX_Trash_Mixer.SFX_Trash_Mixer" (Transformation|GetActorLocation) "0, 0, 0" 1.0 1.0 0.0 "/Game/Game/Actors/ConveyorBelt/Door/SoundDistance.SoundDistance" 0 0 0)
  (bind _newtrack_0 (Timeline|Scaling PlayFromStart)
    (:Update
      (Transformation|SetRelativeScale3D (Variables|Default|GetStaticMesh) _newtrack_0))))

(event EventBeginPlay)

(event Collision|EventActorBeginOverlap
  (params (OtherActor :type Actor%20Object%20Reference)))

(event EventTick
  (params (DeltaSeconds :type Float%20%28single-precision%29)))

(event EventInterfaceInteract
  (params (actor :type Actor%20Object%20Reference) (isHoldingObject :type Boolean) (hitResult :type Hit%20Result%20Structure))
  (bind _asbp_player (Utilities|Casting|CastToBP_Player actor))
  (bind _bp_heldactor (Variables|/Game/Game/Player/BP_Player.BP_Player_C|GetBP_HeldActor _asbp_player)
    (:then
      (Actor|DestroyActor _bp_heldactor))
    (:else)))

(event EventInterfaceObserve
  (params (OwningPlayer :type Actor%20Object%20Reference) (isHoldingObject :type Boolean) (hitResult :type Hit%20Result%20Structure))
  (bind _aswbp_interact_trashbin (Utilities|Casting|CastToWBP_Interact_Trashbin (UserInterface|GetUserWidgetObject (Variables|Default|GetAC_TrashbinWidgetComponent))))
  (Default|ActivateAnimation _aswbp_interact_trashbin))

(fn ConstructionScript)