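; BP_SplinePath is a construction-time path actor that tiles a static mesh along a spline.
; The Construction Script adds X-forward spline mesh components per SectionLength, optionally derived from actor X scale, with configurable collision.
; FullLengthMeshes keeps only whole sections; otherwise one more covers the remainder.
; StartPos and StartPos0 supply each section's local endpoints and tangents, clamping tangent length to the section length.
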(event EventBeginPlay)

(event Collision|EventActorBeginOverlap
  (params (OtherActor :type Actor%20Object%20Reference)))

(event EventTick
  (params (DeltaSeconds :type Float%20%28single-precision%29)))

(fn ConstructionScript
  (if (Variables|SplineSettings|GetAllowScaling)
    (Variables|splineSettings|SetSectionLength (* (.x (Transformation|GetActorScale3D)) 1e+02)))
  (if (Variables|SplineSettings|GetFullLengthMeshes)
    (for _index (range 0 (- (Math|Float|Truncate (/ (Spline|GetSplineLength (Variables|Default|GetSpline)) (Variables|splineSettings|GetSectionLength))) 1))
      (Variables|Default|SetloopIndex _index)
      (bind _returnvalue (AddComponent|AddSplineMeshComponent false))
      (Components|StaticMesh|SetStaticMesh _returnvalue (Variables|splineSettings|GetSplineMesh))
      (SplineMesh|SetForwardAxis _returnvalue "X" true)
      (bind (_newparam1 _newparam2) (CallFunction|StartPos (Variables|Default|GetloopIndex)))
      (bind (_newparam1_2 _newparam2_2) (CallFunction|StartPos0 (Variables|Default|GetloopIndex)))
      (SplineMesh|SetStartandEnd _returnvalue _newparam1 _newparam2 _newparam1_2 _newparam2_2 true :!class /Script/Engine.SplineMeshComponent)
      (Collision|SetCollisionEnabled _returnvalue (Variables|splineSettings|GetCollision)))
    (else
      (for _index_2 (range 0 (Math|Float|Truncate (/ (Spline|GetSplineLength (Variables|Default|GetSpline)) (Variables|splineSettings|GetSectionLength))))
        (Variables|Default|SetloopIndex _index_2)
        (bind _returnvalue_2 (AddComponent|AddSplineMeshComponent false))
        (Components|StaticMesh|SetStaticMesh _returnvalue_2 (Variables|splineSettings|GetSplineMesh))
        (SplineMesh|SetForwardAxis _returnvalue_2 "X" true)
        (bind (_newparam1_3 _newparam2_3) (CallFunction|StartPos (Variables|Default|GetloopIndex)))
        (bind (_newparam1_4 _newparam2_4) (CallFunction|StartPos0 (Variables|Default|GetloopIndex)))
        (SplineMesh|SetStartandEnd _returnvalue_2 _newparam1_3 _newparam2_3 _newparam1_4 _newparam2_4 true :!class /Script/Engine.SplineMeshComponent)
        (Collision|SetCollisionEnabled _returnvalue_2 (Variables|splineSettings|GetCollision))))))

(fn StartPos
  (params (NewParam :type Integer))
  (bind _spline (Variables|Default|GetSpline))
  (bind _sectionlength (Variables|splineSettings|GetSectionLength))
  (bind _returnvalue (* NewParam _sectionlength))
  (return (Spline|GetLocationatDistanceAlongSpline _spline _returnvalue "Local") (Math|Vector|ClampVectorSize (Spline|GetTangentatDistanceAlongSpline _spline _returnvalue "Local") 0.0 (Variables|splineSettings|GetSectionLength))))

(fn StartPos0
  (params (NewParam :type Integer))
  (bind _returnvalue (+ NewParam 1))
  (bind _spline (Variables|Default|GetSpline))
  (bind _sectionlength (Variables|splineSettings|GetSectionLength))
  (bind _returnvalue_2 (* _returnvalue _sectionlength))
  (return (Spline|GetLocationatDistanceAlongSpline _spline _returnvalue_2 "Local") (Math|Vector|ClampVectorSize (Spline|GetTangentatDistanceAlongSpline _spline _returnvalue_2 "Local") 0.0 (Variables|splineSettings|GetSectionLength))))