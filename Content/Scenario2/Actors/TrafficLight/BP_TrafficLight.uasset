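; Traffic light actor that cycles endlessly through green, yellow and red from BeginPlay.
; Timed delays separate the phases, and a LightChange event loops back to the first delay after red.
; Each color function swaps materials on the Green, Yellow and Red components, lighting one and switching the others off.
; The initial appearance is left untouched until the first RedToGreen delay ends.
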(event Custom|LightChange
  ;[0 1 0.8737 0.5] Loops through traffic lights
  (Utilities|FlowControl|Delay (Variables|Default|GetRedToGreen))
  (CallFunction|TurnGreen)
  (Utilities|FlowControl|Delay (Variables|Default|GetGreenToYellow))
  (CallFunction|TurnYellow)
  (Utilities|FlowControl|Delay (Variables|Default|GetYellowToRed))
  (CallFunction|TurnRed)
  (CallFunction|LightChange))

(event EventBeginPlay
  ;[0 1 0.8737 0.5] Loops through traffic lights
  (Utilities|FlowControl|Delay (Variables|Default|GetRedToGreen))
  (CallFunction|TurnGreen)
  (Utilities|FlowControl|Delay (Variables|Default|GetGreenToYellow))
  (CallFunction|TurnYellow)
  (Utilities|FlowControl|Delay (Variables|Default|GetYellowToRed))
  (CallFunction|TurnRed)
  (CallFunction|LightChange))

(event Collision|EventActorBeginOverlap
  (params (OtherActor :type Actor%20Object%20Reference)))

(event EventTick
  (params (DeltaSeconds :type Float%20%28single-precision%29)))

(fn ConstructionScript)

(fn TurnGreen
  ;[0 1 0.6901] Light turns green
  (Rendering|Material|SetMaterial (Variables|Default|GetGreen) 0 "/Game/Scenario2/Actors/TrafficLight/M_GreenLight.M_GreenLight")
  (Rendering|Material|SetMaterial (Variables|Default|GetYellow) 0 "/Game/Scenario2/Actors/TrafficLight/M_LightOff.M_LightOff")
  (Rendering|Material|SetMaterial (Variables|Default|GetRed) 0 "/Game/Scenario2/Actors/TrafficLight/M_LightOff.M_LightOff"))

(fn TurnYellow
  ;[0 1 0.6901] Light turns yellow
  (Rendering|Material|SetMaterial (Variables|Default|GetGreen) 0 "/Game/Scenario2/Actors/TrafficLight/M_LightOff.M_LightOff")
  (Rendering|Material|SetMaterial (Variables|Default|GetYellow) 0 "/Game/Scenario2/Actors/TrafficLight/M_YellowLight.M_YellowLight")
  (Rendering|Material|SetMaterial (Variables|Default|GetRed) 0 "/Game/Scenario2/Actors/TrafficLight/M_LightOff.M_LightOff"))

(fn TurnRed
  ;[0 1 0.6901] Light turns red
  (Rendering|Material|SetMaterial (Variables|Default|GetGreen) 0 "/Game/Scenario2/Actors/TrafficLight/M_LightOff.M_LightOff")
  (Rendering|Material|SetMaterial (Variables|Default|GetYellow) 0 "/Game/Scenario2/Actors/TrafficLight/M_LightOff.M_LightOff")
  (Rendering|Material|SetMaterial (Variables|Default|GetRed) 0 "/Game/Scenario2/Actors/TrafficLight/M_RedLight.M_RedLight"))