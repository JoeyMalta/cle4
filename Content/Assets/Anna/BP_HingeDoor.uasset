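; BP_HingeDoor is a hinged door that swings open and closed continuously from BeginPlay, with no player trigger.
; A Timeline curve drives the Door component's relative yaw.
; When the Timeline finishes, its direction selects OpenDoor or CLoseDoor, which play it from the start or reverse it from the end, forming an endless loop.
; The stored start location feeds only a disconnected SetActorLocation node.
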(event Custom|Open%20Door
  (bind (_direction _newtrack1 _openhingeddoor _opendoorhinge) (Timeline|Timeline PlayFromStart)
    (:Update
      (Transformation|SetRelativeRotation (Variables|Default|GetDoor) (Math|Rotator|MakeRotator 0.0 0.0 _opendoorhinge) false false))
    (:Finished
      (switch Utilities|FlowControl|Switch|SwitchonETimelineDirection _direction
        (:Forward
          (CallFunction|CLoseDoor))
        (:Backward
          (CallFunction|OpenDoor))))))

(event Custom|CLoseDoor
  (bind (_direction _newtrack1 _openhingeddoor _opendoorhinge) (Timeline|Timeline ReverseFromEnd)
    (:Update
      (Transformation|SetRelativeRotation (Variables|Default|GetDoor) (Math|Rotator|MakeRotator 0.0 0.0 _opendoorhinge) false false))
    (:Finished
      (switch Utilities|FlowControl|Switch|SwitchonETimelineDirection _direction
        (:Forward
          (CallFunction|CLoseDoor))
        (:Backward
          (CallFunction|OpenDoor))))))

(event EventBeginPlay
  (Variables|Default|SetStart (Transformation|GetActorLocation))
  (CallFunction|OpenDoor))

(event Collision|EventActorBeginOverlap
  (params (OtherActor :type Actor%20Object%20Reference)))

(event EventTick
  (params (DeltaSeconds :type Float%20%28single-precision%29)))

(fn ConstructionScript)