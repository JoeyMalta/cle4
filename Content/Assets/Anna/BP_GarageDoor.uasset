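; Garage door actor that slides open and closed along a timeline-driven path.
; BeginPlay caches the start location, and the MoveDoor timeline adds its vector track to it to position the actor without sweeping.
; OpenDoor starts a conveyor rolling sound and plays the timeline forward, while CLoseDoor reverses it from the end.
; CallEventFinished runs whenever the timeline finishes.
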(event Custom|Open%20Door
  (Audio|Components|Audio|Play (Variables|Default|GetSFX_ConveyorRolling) 0.0)
  (bind _newtrack1 (Timeline|MoveDoor PlayFromStart)
    (:Update
      (Transformation|SetActorLocation (+ (Variables|Default|GetStartLocation) _newtrack1) false false))
    (:Finished
      (Default|CallEventFinished))))

(event Custom|CLoseDoor
  (bind _newtrack1 (Timeline|MoveDoor ReverseFromEnd)
    (:Update
      (Transformation|SetActorLocation (+ (Variables|Default|GetStartLocation) _newtrack1) false false))
    (:Finished
      (Default|CallEventFinished))))

(event EventBeginPlay
  (Variables|Default|SetStartLocation (Transformation|GetActorLocation)))

(fn ConstructionScript)